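; HUD Blueprint that shows a "Press F to open" prompt and handles the pause menu.
; DrawHUD draws the prompt from the screen center through a gate that the Showtext event opens or closes.
; IsMPressed toggles pause, cursor and input mode, adding a cached MainMenuWidget to the viewport on pause and removing all widgets on resume.
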(event EventShowtext
  (params (showText? :type Boolean))
  ;[1 1 1] showing text
  (if showText?
    (Utilities|FlowControl|Gate true) ; enters at Open
    (else
      (Utilities|FlowControl|Gate true) ; enters at Close
    )))

(event EventDrawHUD
  (params (SizeX :type Integer) (SizeY :type Integer))
  ;[1 1 1] showing text
  (Utilities|FlowControl|Gate true
    (:Exit
      (HUD|DrawText "Press F to open" "(R=0.000000,G=0.000000,B=0.000000,A=1.000000)" (Math|Conversions|ToFloat(Integer) (/ SizeX 2)) (Math|Conversions|ToFloat(Integer) (/ SizeY 2)) "/Game/Character/showTextFont.showTextFont" 0.5 false))))

(event EventIsMPressed
  (params (IsMPressed :type Boolean))
  (bind _returnvalue (Game|GetPlayerController 0))
  ;[1 1 1] Pause menu HUD
  (if IsMPressed
    (Variables|/Script/Engine.PlayerController|SetbShowMouseCursor _returnvalue true)
    (if (== (Variables|Default|GetConfigwidget) 0)
      (bind _returnvalue_2 (UserInterface|CreateWidget "/Game/Blueprints/MainMenuWidget.MainMenuWidget_C"))
      (bind _output_get (Variables|Default|SetConfigwidget _returnvalue_2)))
    (Input|SetInputModeGameandUI _returnvalue 0 false false)
    (UserInterface|Viewport|AddtoViewport _output_get 0)
    (Game|SetGamePaused true)
    (else
      (Variables|/Script/Engine.PlayerController|SetbShowMouseCursor _returnvalue false)
      (Viewport|RemoveAllWidgets)
      (Input|SetInputModeGameOnly _returnvalue)
      (Game|SetGamePaused false))))

(fn ConstructionScript)